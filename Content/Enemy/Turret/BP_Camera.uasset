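; BP_Camera is an enemy camera, filed with turrets, that reacts to the player entering its Box trigger by ending the game.
; Overlap starts a short one-shot Follow Player timer and a looping Fire At Player timer; leaving clears both.
; FollowPlayer turns the Pivot toward player 0, then immediately quits the game.
; No Fire At Player function is defined in this graph.
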(event OnComponentBeginOverlap(Box)
  (params (OverlappedComponent :type Primitive%20Component%20Object%20Reference) (OtherActor :type Actor%20Object%20Reference) (OtherComp :type Primitive%20Component%20Object%20Reference) (OtherBodyIndex :type Integer) (bFromSweep :type Boolean) (SweepResult :type Hit%20Result%20Structure%20%28by%20ref%29))
  (Utilities|Casting|CastToBP_PlayerChar OtherActor)
  (Utilities|Time|SetTimerbyFunctionName 0 "Follow Player" 0.05)
  (Utilities|Time|SetTimerbyFunctionName 0 "Fire At Player" 0.5 true))

(event OnComponentEndOverlap(Box)
  (params (OverlappedComponent :type Primitive%20Component%20Object%20Reference) (OtherActor :type Actor%20Object%20Reference) (OtherComp :type Primitive%20Component%20Object%20Reference) (OtherBodyIndex :type Integer))
  (Utilities|Casting|CastToBP_PlayerChar OtherActor)
  (Utilities|Time|ClearTimerbyFunctionName 0 "Follow Player")
  (Utilities|Time|ClearTimerbyFunctionName 0 "Fire At Player"))

(event Custom|Follow%20Player
  (Transformation|SetWorldRotation (Variables|Default|GetPivot) (Math|Rotator|FindLookatRotation (Transformation|GetActorLocation) (Transformation|GetActorLocation (Game|GetPlayerCharacter 0))) false false)
  (Game|QuitGame 0 "Quit" false))

(fn ConstructionScript)