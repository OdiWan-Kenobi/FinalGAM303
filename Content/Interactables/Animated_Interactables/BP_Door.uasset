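; BP_Door is an interactable door that runs an open timeline on interaction and reverses it three seconds after it finishes.
; INTInteract passes the player to UpdateDoorAngle, whose dot product tests whether they stand in front or behind.
; The timeline lerps the Arrow component's relative Z location, not rotation, toward that result.
; Both sides currently return zero, so that lerp target is always zero.
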(event Custom|ReverseTimeLine
  (bind (_direction _alpha) (Timeline|Timeline Reverse)
    (:Update
      (Transformation|SetRelativeLocation (Variables|Default|GetArrow) (Math|Vector|MakeVector 0.0 0.0 (Math|Float|Lerp 0.0 (stale EventINTInteract _returnvalue) _alpha)) false false))
    (:Finished
      (if (Utilities|Enum|Equal(Enum) _direction "Forward")
        (Utilities|FlowControl|Delay 3.0)
        (CallFunction|ReverseTimeLine)))))

(event EventBeginPlay)

(event Collision|EventActorBeginOverlap
  (params (OtherActor :type Actor%20Object%20Reference)))

(event EventTick
  (params (DeltaSeconds :type Float%20%28single-precision%29)))

(event EventINTInteract
  (params (PlayerRef :type BP%20Player%20Char%20Object%20Reference))
  (bind _returnvalue (CallFunction|UpdateDoorAngle PlayerRef))
  (bind (_direction _alpha) (Timeline|Timeline Play)
    (:Update
      (Transformation|SetRelativeLocation (Variables|Default|GetArrow) (Math|Vector|MakeVector 0.0 0.0 (Math|Float|Lerp 0.0 _returnvalue _alpha)) false false))
    (:Finished
      (if (Utilities|Enum|Equal(Enum) _direction "Forward")
        (Utilities|FlowControl|Delay 3.0)
        (CallFunction|ReverseTimeLine)))))

(fn ConstructionScript)

(fn UpdateDoorAngle
  (params (self2 :type Actor%20Object%20Reference))
  (return (select (> (Math|Vector|DotProduct (Math|Vector|GetUnitDirection(Vector) (Transformation|GetActorLocation) (Transformation|GetActorLocation self2)) (Transformation|GetActorForwardVector)) 0.0) 0.0 0.0)))