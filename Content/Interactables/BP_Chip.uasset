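; BP_Chip is an interactable colored cube that the player can pick up and drop, and picking it up quits the game.
; An interact event checks and sets the player's IsHolding flag, disables Cube physics and collision, attaches it to Arrow1, then calls QuitGame.
; A drop event detaches the actor and restores collision and physics.
; The construction script tints the cube through a dynamic material instance using PickupColor.
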(event EventINTInteract
  (params (PlayerRef :type BP%20Player%20Char%20Object%20Reference))
  (bind _cube (Variables|Default|GetCube))
  ;[0.15 0.15 0.15 0.5] Pick up
  (if (not (Variables|/Game/Player/BP_PlayerChar.BP_PlayerChar_C|GetisHolding? PlayerRef))
    (Variables|/Game/Player/BP_PlayerChar.BP_PlayerChar_C|SetisHolding? PlayerRef true)
    (Physics|SetSimulatePhysics _cube false)
    (Collision|SetCollisionEnabled _cube "NoCollision")
    (Transformation|AttachComponentToComponent (Variables|Default|GetCube) (Variables|/Game/Player/BP_PlayerChar.BP_PlayerChar_C|GetArrow1 PlayerRef) "None" "SnapToTarget" "KeepRelative" "KeepRelative" true)
    (Game|QuitGame 0 "Quit" false)))

(event EventINTDrop
  (bind _cube (Variables|Default|GetCube))
  ;[0.15 0.15 0.15 0.5] Drop
  (Transformation|DetachFromActor "KeepWorld" "KeepWorld" "KeepWorld")
  (Collision|SetCollisionEnabled _cube "QueryAndPhysics")
  (Physics|SetSimulatePhysics _cube true))

(fn ConstructionScript
  (bind _returnvalue (Rendering|Material|CreateDynamicMaterialInstance (Variables|Default|GetCube) 0 "/Game/Interactables/Animated_Interactables/MAT_color.MAT_color" "None" :!class /Script/Engine.PrimitiveComponent))
  (bind _output_get (Variables|Default|SetColorDMI _returnvalue))
  (Rendering|Material|SetVectorParameterValue _output_get "Color" (Variables|Default|GetPickupColor) :!class /Script/Engine.MaterialInstanceDynamic))